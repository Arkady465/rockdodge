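; BP_RockSpawner is a spawner actor that drops BP_Rock actors at random points within its Box area.
; On BeginPlay it reads the difficulty from BP_RockDodgeGameInstances and sets BaseRockDamage for Easy, Medium or Hard.
; The SpawnRockInVolume event randomizes X and Y inside the box, keeps the spawner's Z and always spawns regardless of collision.
; Nothing here triggers that event or passes the damage value to spawned rocks.
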(event `self.ReceiveBeginPlay`
  (bind _asbp_rock_dodge_game_instances (cast `/Game/RockDodge/Core/GameInstances/BP_RockDodgeGameInstances` (`GameplayStatics.GetGameInstance`)))
  (set `self.BaseRockDamage` (select `/Game/RockDodge/Core/Enums/EGameDifficulty` (`/Game/RockDodge/Core/GameInstances/BP_RockDodgeGameInstances.GetGameDifficulty` _asbp_rock_dodge_game_instances) :`NewEnumerator0` 15.0 :`NewEnumerator1` 40.0 :`NewEnumerator2` 100.0)))

(event `SpawnRockInVolume`
  (bind _box (`self.Box`))
  (`|SpawnActorFromClass` "/Game/RockDodge/Blueprints/BP_Rock.BP_Rock_C" (`KismetMathLibrary.MakeTransform` (`KismetMathLibrary.MakeVector` (.x (`KismetMathLibrary.RandomPointInBoundingBox` (`SceneComponent.K2_GetComponentLocation` _box) (`BoxComponent.GetScaledBoxExtent` _box))) (.y (`KismetMathLibrary.RandomPointInBoundingBox` (`SceneComponent.K2_GetComponentLocation` _box) (`BoxComponent.GetScaledBoxExtent` _box))) (.z (`self.K2_GetActorLocation`)))) "AlwaysSpawn" "OverrideRootScale" null null))

(fn `UserConstructionScript`)