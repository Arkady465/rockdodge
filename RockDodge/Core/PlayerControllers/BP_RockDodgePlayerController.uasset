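; Player controller for Rock Dodge that drives movement and look for BP_RockDodgerCharacter through Enhanced Input.
; On BeginPlay it sets game-only input with a visible cursor, adds the IMC_DodgeRock mapping context, and caches the pawn's movement component.
; Move input feeds that component directly along control-rotation forward and right vectors, while look input adds yaw and pitch.
; NewFunction is an unused stub.
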(event `self.ReceiveBeginPlay`
  (`WidgetBlueprintLibrary.SetInputMode_GameOnly` self)
  (set `self.bShowMouseCursor` true)
  (`EnhancedInputSubsystemInterface.AddMappingContext` (subsystem `EnhancedInputLocalPlayerSubsystem`) "/Game/RockDodge/Core/EnhancedInput/IMC_DodgeRock.IMC_DodgeRock" 0 (struct))
  (bind _asbp_rock_dodger_character (cast `/Game/RockDodge/Characters/BP_RockDodgerCharacter` (`self.K2_GetPawn`)))
  (bind _output_get (set `self.RockDodgerCharacter` _asbp_rock_dodger_character))
  (set `self.Character Movement` (`Character.CharacterMovement` _output_get)))

(event `EnhancedInput|/Game/RockDodge/Core/EnhancedInput/Action/IA_DodgeRockMove`
  (params (ActionValue :type "Vector2D Structure") (ElapsedSeconds :type "Float (double-precision)") (TriggeredSeconds :type "Float (double-precision)") (InputAction :type "InputAction Object Reference" :default "/Game/RockDodge/Core/EnhancedInput/Action/IA_DodgeRockMove.IA_DodgeRockMove"))
  (bind (_returnvalue_roll _returnvalue_pitch _returnvalue_yaw) (`KismetMathLibrary.BreakRotator` (`self.GetControlRotation`)))
  (bind (_returnvalue_roll_2 _returnvalue_pitch_2 _returnvalue_yaw_2) (`KismetMathLibrary.BreakRotator` (`self.GetControlRotation`)))
  (:`Triggered`
    (bind _character_movement (`self.Character Movement`)
      (:`then`
        (`|ExecutionSequence`
          (:`then_0`
            (`PawnMovementComponent.AddInputVector` _character_movement (* (`KismetMathLibrary.GetForwardVector` (`KismetMathLibrary.MakeRotator` 0.0 0.0 _returnvalue_yaw)) ActionValue_Y) false))
          (:`then_1`
            (`PawnMovementComponent.AddInputVector` _character_movement (* (`KismetMathLibrary.GetRightVector` (`KismetMathLibrary.MakeRotator` _returnvalue_roll_2 0.0 _returnvalue_yaw_2)) ActionValue_X) false))))
      (:`else`))))

(event `EnhancedInput|/Game/RockDodge/Core/EnhancedInput/Action/IA_DodgeRockLook`
  (params (ActionValue :type "Vector2D Structure") (ElapsedSeconds :type "Float (double-precision)") (TriggeredSeconds :type "Float (double-precision)") (InputAction :type "InputAction Object Reference" :default "/Game/RockDodge/Core/EnhancedInput/Action/IA_DodgeRockLook.IA_DodgeRockLook"))
  (:`Triggered`
    (`self.AddYawInput` ActionValue_X)
    (`self.AddPitchInput` ActionValue_Y)))

(fn `NewFunction`
  (params (A :type "Vector Structure")))

(fn `UserConstructionScript`)