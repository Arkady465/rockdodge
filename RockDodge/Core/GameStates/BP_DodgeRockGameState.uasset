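; Game state for Rock Dodge that runs the match timer, score updates, game end and level reload.
; A looping one-second timer advances TimePlayed by 3, zeroes RockCount before adding it to player score, and passes the time to the game mode's Process.
; EndGame stops the timer, sends the score to the game instance as highest score, then calls the game mode's RestartGame after a delay.
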(event `self.ReceiveBeginPlay`
  (`|ExecutionSequence`
    (:`then_0`
      (bind _asbp_dodge_rock_player_state (cast `/Game/RockDodge/Core/PlayerStates/BP_DodgeRockPlayerState` (`GameplayStatics.GetPlayerState` 0)))
      (set `self.DodgeRockPlayerState` _asbp_dodge_rock_player_state))
    (:`then_1`
      (bind _asbp_dodge_rock_game_mode (cast `/Game/RockDodge/Core/GameModes/BP_DodgeRockGameMode` (`GameplayStatics.GetGameMode`)))
      (set `self.DodgeRockGameMode` _asbp_dodge_rock_game_mode))))

(event `StartGame`
  (bind _returnvalue (`KismetSystemLibrary.K2_SetTimerDelegate` (`|CreateDelegate` self :!event `CoreGameTimerEvent`) 1.0 true))
  (set `self.CoreGameTimer` _returnvalue)
  (set `self.IsGameEnded?` false))

(event `EndGame`
  (`KismetSystemLibrary.K2_ClearAndInvalidateTimerHandle` (`self.CoreGameTimer`))
  (set `self.IsGameEnded?` true)
  (`|ExecutionSequence`
    (:`then_0`
      (bind _asbp_rock_dodge_game_instances (cast `/Game/RockDodge/Core/GameInstances/BP_RockDodgeGameInstances` (`GameplayStatics.GetGameInstance`)))
      (bind _dodgerockplayerstate (`self.DodgeRockPlayerState`)
        (:`then`
          (`/Game/RockDodge/Core/GameInstances/BP_RockDodgeGameInstances.SetHighestScore` _asbp_rock_dodge_game_instances (`/Game/RockDodge/Core/PlayerStates/BP_DodgeRockPlayerState.GetPlayerScore` _dodgerockplayerstate) null))
        (:`else`)))
    (:`then_1`
      (`KismetSystemLibrary.Delay` 3.0)
      (bind _dodgerockgamemode (`self.DodgeRockGameMode`)
        (:`then`
          (`/Game/RockDodge/Core/GameModes/BP_DodgeRockGameMode.RestartGame` _dodgerockgamemode))
        (:`else`)))))

(event `RestartGame`
  (bind _returnvalue (`GameplayStatics.GetCurrentLevelName` true))
  (`GameplayStatics.OpenLevel` (`KismetStringLibrary.Conv_StringToName` _returnvalue)))

(event `CoreGameTimerEvent`
  (set `self.TimePlayed` (+ 3 (`self.TimePlayed`)))
  (`|ExecutionSequence`
    (:`then_0`
      (bind _dodgerockplayerstate (`self.DodgeRockPlayerState`)
        (:`then`
          (bind _output_get (set `self.RockCount` 0))
          (`/Game/RockDodge/Core/PlayerStates/BP_DodgeRockPlayerState.SetPlayerScore` _dodgerockplayerstate (+ (`/Game/RockDodge/Core/PlayerStates/BP_DodgeRockPlayerState.GetPlayerScore` _dodgerockplayerstate) _output_get)))
        (:`else`)))
    (:`then_1`
      (bind _dodgerockgamemode (`self.DodgeRockGameMode`)
        (:`then`
          (`/Game/RockDodge/Core/GameModes/BP_DodgeRockGameMode.Process` _dodgerockgamemode (`self.TimePlayed`)))
        (:`else`)))))

(fn `GetRockCount`
  (returns (RockCount :type Integer))
  (return (`self.RockCount`)))

(fn `SetRockCount`
  (params (RockCount :type Integer))
  (set `self.RockCount` RockCount))

(fn `UserConstructionScript`)