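; Game Instance Blueprint for RockDodge that holds the selected game difficulty and the highest score.
; Simple getter and setter functions expose both values.
; The high-score setter stores a new score only if a passed-in target object is valid and the score beats the value that target returns from GetHighestScore.
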(fn `GetGameDifficulty`
  (returns (GameDifficulty :type "/Game/RockDodge/Core/Enums/EGameDifficulty Enum"))
  (return (`self.GameDifficulty`)))

(fn `GetHighestScore`
  (returns (HighestScore :type Integer))
  (return (`self.HighestScore`)))

(fn `SetGameDifficulty`
  (params (GameDifficulty :type "/Game/RockDodge/Core/Enums/EGameDifficulty Enum" :default "NewEnumerator0"))
  (set `self.GameDifficulty` GameDifficulty))

(fn `SetHighestScore`
  (params (HighestScore :type Integer) (`Цель` :type "Self Object Reference"))
  (`/Engine/EditorBlueprintResources/StandardMacros.IsValid` `Цель`
    (:`Is Valid`
      (bind _highestscore (`self.GetHighestScore` `Цель`))
      (if (> HighestScore _highestscore)
        (set `self.HighestScore` HighestScore)))))