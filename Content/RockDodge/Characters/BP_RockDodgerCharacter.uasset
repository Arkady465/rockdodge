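; Player character for the RockDodge game, with jump input and a ragdoll death.
; When its health component reports death, it disables player input and capsule collision, turns on spring arm collision testing and makes the mesh simulate physics.
; While dead, Tick moves the actor to the simulated mesh's location each frame, so the actor follows the ragdoll.
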(event `EnhancedInput|/Game/RockDodge/Core/EnhancedInput/Action/IA_DodgeRockJump`
  (params (ActionValue :type Boolean) (ElapsedSeconds :type "Float (double-precision)") (TriggeredSeconds :type "Float (double-precision)") (InputAction :type "InputAction Object Reference" :default "/Game/RockDodge/Core/EnhancedInput/Action/IA_DodgeRockJump.IA_DodgeRockJump"))
  (:`Triggered`
    (`self.Jump`))
  (:`Canceled`
    (`self.StopJumping`)))

(event `self.BP_HealthComponent.OnOwnerDied`
  (bind _mesh (`self.Mesh`))
  (set `self.IsDead?` true)
  (`self.DisableInput` (`GameplayStatics.GetPlayerController` 0))
  (set `SpringArmComponent.bDoCollisionTest` true (`self.SpringArm`))
  (`PrimitiveComponent.SetCollisionEnabled` (`self.CapsuleComponent`) "NoCollision")
  (`PrimitiveComponent.SetCollisionEnabled` _mesh "QueryAndPhysics")
  (`PrimitiveComponent.SetSimulatePhysics` _mesh true))

(event `self.ReceiveTick`
  (params (DeltaSeconds :type "Float (single-precision)"))
  (if (`self.IsDead?`)
    (`self.K2_SetActorLocation` (`SceneComponent.K2_GetComponentLocation` (`self.Mesh`)))))

(fn `UserConstructionScript`)